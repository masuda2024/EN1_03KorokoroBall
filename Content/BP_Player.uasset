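; BP_Player is a player Blueprint that is set up to push a Sphere component with physics force from Enhanced Input.
; BeginPlay adds the IMC_InGame mapping context, and one IA_Move handler prints the input value.
; A second IA_Move handler scales input by delta time and Acceleration, then normalizes it for AddForce, discarding that magnitude.
; It multiplies the right and forward axis vectors instead of adding them, so the force resolves to zero.
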(event `EnhancedInput|/Game/IA_Move`
  (params (ActionValue :type "Vector2D Structure") (ElapsedSeconds :type "Float (double-precision)") (TriggeredSeconds :type "Float (double-precision)") (InputAction :type "InputAction Object Reference" :default "/Game/IA_Move.IA_Move"))
  (:`Triggered`
    (`KismetSystemLibrary.PrintString` (`KismetStringLibrary.Conv_Vector2dToString` ActionValue))))

(event `EnhancedInput|/Game/IA_Move`
  (params (ActionValue :type "Vector2D Structure") (ElapsedSeconds :type "Float (double-precision)") (TriggeredSeconds :type "Float (double-precision)") (InputAction :type "InputAction Object Reference" :default "/Game/IA_Move.IA_Move"))
  (bind (_x _y) (`KismetMathLibrary.BreakVector2D` (* ActionValue (* (`GameplayStatics.GetWorldDeltaSeconds`) (`self.Acceleration`)))))
  (:`Triggered`
    (`PrimitiveComponent.AddForce` (`self.Sphere`) (`KismetMathLibrary.Normal` (* (* (`KismetMathLibrary.Vector_Right`) _x) (* (`KismetMathLibrary.Vector_Forward`) _y))) "None" false)))

(event `self.ReceiveBeginPlay`
  (`EnhancedInputSubsystemInterface.AddMappingContext` (pcsubsystem `EnhancedInputLocalPlayerSubsystem` (`GameplayStatics.GetPlayerController` 0)) "/Game/IMC_InGame.IMC_InGame" 0 (struct)))

(fn `UserConstructionScript`)